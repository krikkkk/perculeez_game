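; BP_CharacterData is a Blueprint Interface that exposes a fighting game character's state through getter functions.
; It groups the data into base transform, player name, character setup, movement inputs, health, locomotion and fighting state, including combos, defense, knockdown and match outcome.
; The functions hold no logic and return only defaults, leaving the actual values to implementing classes.
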(fn `Get Base Data`
  (returns (`Actor Rotation` :type "Rotator Structure") (`Actor Location` :type "Vector Structure"))
  (return (struct) (0.0 0.0 0.0)))

(fn `Get Character Data`
  (returns (Character :type "/Game/Blueprints/Data/Struc/S_Character_Data Structure") (`Character Type` :type "/Game/Blueprints/Data/Enum/E_Character_Type Enum") (`Max Health` :type Integer) (`Max Combo Value` :type Integer) (`Default Material` :type "Array of MaterialInstance Object Reference") (`Character Material Last Index` :type Integer) (`Character Intro Material` :type "MaterialInstance Object Reference") (`Animations Play Rate` :type "Float (double-precision)") (`Hit Duration` :type "Float (double-precision)"))
  (return (struct) "NewEnumerator0" 0 0 _ 0 null 0.0 0.0))

(fn `Get Health & Damage`
  (returns (`Is Dead` :type Boolean) (Health :type Integer))
  (return false 0))

(fn `Get Inputs`
  (returns (`Move Right` :type "Float (double-precision)") (`Move Forward` :type "Float (double-precision)") (`Can Jump` :type Boolean))
  (return 0.0 0.0 false))

(fn `Get Locomotion`
  (returns (`On Ground` :type Boolean) (`In Air` :type Boolean) (Jumped :type Boolean) (Crouch :type Boolean) (Speed :type "Float (double-precision)"))
  (return false false false false 0.0))

(fn `Get Player Data`
  (returns (`Player Name` :type Name) (`Player Image` :type "Texture2D Object Reference"))
  (return "None" null))

(fn `GetFighting Data`
  (returns (`Playing Montage` :type Boolean) (`Knocked Down` :type Boolean) (Defend :type Boolean) (`Hit Data` :type "/Game/Blueprints/Data/Struc/S_Hit_Data Structure") (`Is Hitting` :type Boolean) (Combo :type Boolean) (`Combo Level` :type "/Game/Blueprints/Data/Enum/E_Combo_Level Enum") (`Combo Value` :type Integer) (Finish :type Boolean) (`Player Lost The Game` :type Boolean) (`Enable Hits` :type Boolean))
  (return false false false (struct) false false "NewEnumerator3" 0 false false false))