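; BP_AI_Master is an AI-controlled fighter that attacks, defends and advances on BP_Player.
; A self-rescheduling timer fires at random intervals to hit when the player is reachable and the game has started, and to randomly toggle brief defending and movement.
; Each tick, a capsule trace at FinishEnemyLocation sets CanHitEnemy, and the AI moves along its MoveRight axis only when out of range and allowed to move.
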(event `self.ReceiveBeginPlay`
  (`parent.ReceiveBeginPlay`)
  ;[1 1 1] AI_Functions
  (`KismetSystemLibrary.K2_SetTimerDelegate` (delegate `AI_Functions`) (`KismetMathLibrary.RandomFloatInRange` 0.2 1.0) true :!label _label))

(event `AI_Functions`
  (bind _returnvalue (`KismetMathLibrary.RandomBool`))
  (bind _returnvalue_2 (select `bool` (`self.Finish`) :`false` (select `bool` (`self.Combo`) :`false` (select `bool` _returnvalue :`false` "NewEnumerator0" :`true` "NewEnumerator1" :!type "/Game/Blueprints/Data/Enum/E_Hit_Type Enum") :`true` "NewEnumerator2") :`true` "NewEnumerator3"))
  ;[1 1 1] AI_Functions
  (`|ExecutionSequence`
    (:`then_0`
      (goto _label))
    (:`then_1`
      (if (`self.Can Hit Enemy`)
        (if (`self.Game Started`)
          (`self.Hit` _returnvalue_2 (select `/Game/Blueprints/Data/Enum/E_Hit_Type` _returnvalue_2 :`NewEnumerator0` (select `bool` _returnvalue :`false` (select `bool` _returnvalue :`false` "NewEnumerator0" :`true` "NewEnumerator1" :!type "/Game/Anim/Data/Enum/E_Bones Enum") :`true` (select `bool` _returnvalue :`false` "NewEnumerator4" :`true` "NewEnumerator5" :!type "/Game/Anim/Data/Enum/E_Bones Enum")) :`NewEnumerator1` (select `bool` _returnvalue :`false` "NewEnumerator2" :`true` "NewEnumerator3" :!type "/Game/Anim/Data/Enum/E_Bones Enum") :`NewEnumerator2` "NewEnumerator6" :`NewEnumerator3` "NewEnumerator6")))))
    (:`then_2`
      (bind _output_get (set `self.Defend` (`KismetMathLibrary.RandomBool`)))
      (if _output_get
        (`KismetSystemLibrary.Delay` (`KismetMathLibrary.RandomFloatInRange` 0.2 1.0))
        (set `self.Defend` false)))
    (:`then_3`
      (if (`KismetMathLibrary.RandomBool`)
        _))
    (:`then_4`
      (set `self.AI can Move` (`KismetMathLibrary.RandomBool`)))))

(event `self.ReceiveTick`
  (params (DeltaSeconds :type "Float (single-precision)"))
  ;[1 1 1] Update
  (`parent.ReceiveTick` DeltaSeconds)
  (`self.Check if AI can Hit Enemy`)
  (`self.AI Move To Enemy`))

(fn `AI Move To Enemy`
  ;[1 1 1] AI Move To Enemy
  (`self.MoveRight` (select `bool` (or (`self.Can Hit Enemy`) (not (`self.AI can Move`))) :`false` 1.0)))

(fn `Check if AI can Hit Enemy`
  (bind _capsulecomponent (`self.CapsuleComponent`))
  (bind _returnvalue (`SceneComponent.K2_GetComponentLocation` (`self.Finish Enemy Location`)))
  ;[1 1 1] Check if AI can Hit Enemy
  (bind (_outhit _returnvalue_2) (`KismetSystemLibrary.CapsuleTraceSingle` _returnvalue _returnvalue (`CapsuleComponent.CapsuleRadius` _capsulecomponent) (`CapsuleComponent.CapsuleHalfHeight` _capsulecomponent) "TraceTypeQuery3"))
  (if _returnvalue_2
    (cast `/Game/Blueprints/BP_Player` (`.HitActor` (`GameplayStatics.BreakHitResult` _outhit))
      (:`then`
        (set `self.Can Hit Enemy` true))
      (:`CastFailed`
        (set `self.Can Hit Enemy` false :!label _label)))
    (else
      (goto _label))))

(fn `UserConstructionScript`
  (`parent.UserConstructionScript`))