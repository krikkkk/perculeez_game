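; Main Game Instance that holds fight data and handles level travel, the settings menu, confirmation popups and graphics settings.
; StartFight optionally stores FightingData and opens its map, while OpenLevel maps an enum to the main menu or test map.
; It creates and toggles the settings widget and spawns selection messages whose Yes/No actions are enum-driven.
; Scalability helpers translate between quality levels and GameUserSettings, which ApplySettings applies and saves.
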(event `/Game/Blueprints/Data/Interfaces/Events/GameInstance/BPI_GameInstance_Events.Start Fight`
  (params (`Set New Data` :type Boolean) (`Fighting Data` :type "/Game/Blueprints/Data/Struc/S_Fighting_Data Structure"))
  ;[1 1 1] Change FightingData
  (`|ExecutionSequence`
    (:`then_0`
      (if `Set New Data`
        (set `self.Fighting Data` `Fighting Data`)))
    (:`then_1`
      (`/Game/Blueprints/Data/Interfaces/Events/GameInstance/BPI_GameInstance_Events.OpenLevel` self (`.Map_8_FD5ECE8E42446C70C36BB0A711977888` (break `/Game/Blueprints/Data/Struc/S_Map_Data` (`.Map_11_000EC4C143D9F69045525EA59526AFF2` (break `/Game/Blueprints/Data/Struc/S_Fighting_Data` `Fighting Data`))))))))

(event `/Game/Blueprints/Data/Interfaces/Events/GameInstance/BPI_GameInstance_Events.OpenLevel`
  (params (Map :type "/Game/Blueprints/Data/Enum/E_Maps Enum" :default "NewEnumerator1"))
  ;[1 1 1] Open Level
  (`GameplayStatics.OpenLevelBySoftObjectPtr` (select `/Game/Blueprints/Data/Enum/E_Maps` Map :`NewEnumerator1` "/Game/Maps/L_MainMenu.L_MainMenu" :`NewEnumerator0` "/Game/Maps/Test_Maps/L_Test_Map.L_Test_Map" :!type "World Soft Object Reference")))

(event `/Game/Blueprints/Data/Interfaces/Events/GameInstance/BPI_GameInstance_Events.OpenSettings`
  (params (OwningPlayer :type "PlayerController Object Reference"))
  ;[1 1 1] Open Settings
  (bind _output_get (set `self.IsOpen Settings` (not (`self.IsOpen Settings`))))
  (bind _settings_widget (`self.Settings Widget`)
    (:`then`
      (`Widget.SetVisibility` _settings_widget (select `bool` _output_get :`false` "Hidden" :`true` "Visible" :!type "ESlateVisibility Enum")))
    (:`else`
      (if _output_get
        (bind _returnvalue (`|CreateWidget` "/Game/Blueprints/UI/Settings/WB_Settings.WB_Settings_C" OwningPlayer))
        (bind _output_get_2 (set `self.Settings Widget` _returnvalue))
        (`UserWidget.AddToViewport` _output_get_2 0)))))

(event `/Game/Blueprints/Data/Interfaces/Events/GameInstance/BPI_GameInstance_Events.Create Selection Message`
  (params (OwningPlayer :type "PlayerController Object Reference") (Message :type Text) (`Yes Function` :type "/Game/Blueprints/Data/Enum/Widget/E_Message_Function Enum" :default "NewEnumerator1") (`No Function` :type "/Game/Blueprints/Data/Enum/Widget/E_Message_Function Enum" :default "NewEnumerator1"))
  ;[1 1 1] Selection Message
  ;;[1 1 1] Create Selection Message
  (bind _returnvalue (`|CreateWidget` "/Game/Blueprints/UI/Custom/WB_SelectionMessage.WB_SelectionMessage_C" OwningPlayer Message `Yes Function` `No Function`))
  (bind _output_get (set `self.Selection Message Widget` _returnvalue))
  (`UserWidget.AddToViewport` _output_get 0))

(event `/Game/Blueprints/Data/Interfaces/Events/GameInstance/BPI_GameInstance_Events.Selection Message Functions`
  (params (`Yes Selection` :type Boolean) (`Yes Function` :type "/Game/Blueprints/Data/Enum/Widget/E_Message_Function Enum" :default "NewEnumerator1") (`No Function` :type "/Game/Blueprints/Data/Enum/Widget/E_Message_Function Enum" :default "NewEnumerator1"))
  ;[1 1 1] Selection Message
  ;;[1 1 1] Selection Message Function
  (if `Yes Selection`
    (switch `/Game/Blueprints/Data/Enum/Widget/E_Message_Function` `Yes Function`
      (:`NewEnumerator1`
        (bind _selection_message_widget (`self.Selection Message Widget` :!label _label)
          (:`then`
            (`Widget.RemoveFromParent` _selection_message_widget))
          (:`else`)))
      (:`NewEnumerator0`
        (`KismetSystemLibrary.QuitGame` null "Quit" :!label _label_2)))
    (else
      (switch `/Game/Blueprints/Data/Enum/Widget/E_Message_Function` `No Function`
        (:`NewEnumerator1`
          (goto _label))
        (:`NewEnumerator0`
          (goto _label_2))))))

(event `/Game/Blueprints/Data/Interfaces/Events/GameInstance/BPI_GameInstance_Events.ChangeScalibilitySettings`
  (params (ScalabilitySetting :type "/Game/Blueprints/Data/Enum/Widget/Settings/E_ScalabilitySettings Enum" :default "NewEnumerator0") (ScalabilityLevel :type "/Game/Blueprints/Data/Enum/Widget/Settings/E_ScalabilityLevel Enum" :default "NewEnumerator1"))
  ;[1 1 1] Change Scalability Setting
  (`self.Change Scalability Setting` ScalabilitySetting (select `/Game/Blueprints/Data/Enum/Widget/Settings/E_ScalabilityLevel` ScalabilityLevel :`NewEnumerator2` 1 :`NewEnumerator3` 2 :`NewEnumerator4` 3 :`NewEnumerator5` 4)))

(event `/Game/Blueprints/Data/Interfaces/Events/GameInstance/BPI_GameInstance_Events.ApplySettings`
  ;[1 1 1] Apply Settings
  (bind _returnvalue (`GameUserSettings.GetGameUserSettings`))
  (`|ExecutionSequence`
    (:`then_0`
      (`GameUserSettings.ApplySettings` _returnvalue true))
    (:`then_1`
      (`GameUserSettings.SaveSettings` _returnvalue))))

(fn `Change Scalability Setting`
  (params (Setting :type "/Game/Blueprints/Data/Enum/Widget/Settings/E_ScalabilitySettings Enum" :default "NewEnumerator0") (Level :type Integer))
  ;[1 1 1] Change Scalability Setting
  (bind _returnvalue (`GameUserSettings.GetGameUserSettings`))
  (switch `/Game/Blueprints/Data/Enum/Widget/Settings/E_ScalabilitySettings` Setting
    (:`NewEnumerator1`
      (`GameUserSettings.SetViewDistanceQuality` _returnvalue Level))
    (:`NewEnumerator2`
      (`GameUserSettings.SetAntiAliasingQuality` _returnvalue Level))
    (:`NewEnumerator3`
      (`GameUserSettings.SetPostProcessingQuality` _returnvalue Level))
    (:`NewEnumerator4`
      (`GameUserSettings.SetShadowQuality` _returnvalue Level))
    (:`NewEnumerator5`
      (`GameUserSettings.SetGlobalIlluminationQuality` _returnvalue Level))
    (:`NewEnumerator6`
      (`GameUserSettings.SetReflectionQuality` _returnvalue Level))
    (:`NewEnumerator7`
      (`GameUserSettings.SetTextureQuality` _returnvalue Level))
    (:`NewEnumerator8`
      (`GameUserSettings.SetVisualEffectQuality` _returnvalue Level))
    (:`NewEnumerator9`
      (`GameUserSettings.SetFoliageQuality` _returnvalue Level))
    (:`NewEnumerator10`
      (`GameUserSettings.SetShadingQuality` _returnvalue Level))))

(fn `Get Game Refs`
  (returns (`Game Instance` :type "/Game/Blueprints/Base/BP_Main_GameInstance Object Reference") (`Game Mode` :type "/Game/Blueprints/Base/GameMode/BP_Main_GameMode Object Reference") (`Game State` :type "/Game/Blueprints/Base/BP_Main_GameState Object Reference") (`Player Controller` :type "/Game/Blueprints/Base/BP_Main_PlayerController Object Reference") (`Camera Manager` :type "/Game/Blueprints/Base/BP_Main_CameraManager Object Reference") (`Player State` :type "/Game/Blueprints/Base/BP_Main_PlayerState Object Reference") (Player :type "/Game/Blueprints/BP_Player Object Reference") (Enemy :type "/Game/Blueprints/BP_Player Object Reference"))
  (return null null null null null null null null))

(fn `Get GameInstance data`
  (returns (`Fighting Data` :type "/Game/Blueprints/Data/Struc/S_Fighting_Data Structure"))
  (return (`self.Fighting Data`)))

(fn `Get GameMode Data`
  (returns (`Fighting Data` :type "/Game/Blueprints/Data/Struc/S_Fighting_Data Structure") (`Game Started` :type Boolean) (Timer :type Integer) (`Game Ended` :type Boolean))
  (return (struct) false 0 false))

(fn `Get GameState Data`
  (returns (`Game Time` :type "Timecode Structure"))
  (return))

(fn `Get Setting Level`
  (params (Setting :type "/Game/Blueprints/Data/Enum/Widget/Settings/E_ScalabilitySettings Enum" :default "NewEnumerator0"))
  (returns (`Setting Level` :type "/Game/Blueprints/Data/Enum/Widget/Settings/E_ScalabilityLevel Enum"))
  ;[1 1 1] Get Setting Level
  (bind _returnvalue (`GameUserSettings.GetGameUserSettings`))
  (return (select `int` (select `/Game/Blueprints/Data/Enum/Widget/Settings/E_ScalabilitySettings` Setting :`NewEnumerator1` (`GameUserSettings.GetViewDistanceQuality` _returnvalue) :`NewEnumerator2` (`GameUserSettings.GetAntiAliasingQuality` _returnvalue) :`NewEnumerator3` (`GameUserSettings.GetPostProcessingQuality` _returnvalue) :`NewEnumerator4` (`GameUserSettings.GetShadowQuality` _returnvalue) :`NewEnumerator5` (`GameUserSettings.GetGlobalIlluminationQuality` _returnvalue) :`NewEnumerator6` (`GameUserSettings.GetReflectionQuality` _returnvalue) :`NewEnumerator7` (`GameUserSettings.GetTextureQuality` _returnvalue) :`NewEnumerator8` (`GameUserSettings.GetVisualEffectQuality` _returnvalue) :`NewEnumerator9` (`GameUserSettings.GetFoliageQuality` _returnvalue) :`NewEnumerator10` (`GameUserSettings.GetShadingQuality` _returnvalue)) :`0` "NewEnumerator1" :`1` "NewEnumerator2" :`2` "NewEnumerator3" :`3` "NewEnumerator4" :`4` "NewEnumerator5" :`5` "NewEnumerator6" :!type "/Game/Blueprints/Data/Enum/Widget/Settings/E_ScalabilityLevel Enum")))