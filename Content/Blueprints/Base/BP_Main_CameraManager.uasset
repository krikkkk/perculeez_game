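; Player camera manager that frames the fight between player and enemy, caching both actors' transforms each tick through message calls.
; BlueprintUpdateCamera offsets from their raised midpoint along the player's forward axis by a separation-based distance, then smoothly interpolates position and yaw-only look-at.
; A camera trace pulls the view to any obstruction and flips sides, with a two-second cooldown, when the hit lies within CameraLength of the desired position.
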(event `self.ReceiveTick`
  (params (DeltaSeconds :type "Float (single-precision)"))
  ;[1 1 1] Update
  (`self.Get Refs`)
  (`self.Get Player Data`)
  (`self.Get Enemy Data`))

(event `Switch Camera`
  ;[1 1 1] Switch Camera
  (`/Engine/EditorBlueprintResources/StandardMacros.DoOnce` false :!label _label
    (:`Completed`
      (set `self.Switch Camera Side` (not (`self.Switch Camera Side`)))
      (`KismetSystemLibrary.Delay` 2.0)
      (goto _label :!via `Reset`))))

(fn `BlueprintUpdateCamera`
  (params (CameraTarget :type "Actor Object Reference"))
  (returns (NewCameraLocation :type "Vector Structure") (NewCameraRotation :type "Rotator Structure") (NewCameraFOV :type "Float (single-precision)") (ReturnValue :type Boolean))
  (bind _camera_length (`self.Camera Length`))
  (bind _enemy_location (`self.Enemy Location`))
  (bind _player_location (`self.Player Location`))
  (bind _returnvalue (`KismetMathLibrary.Vector_Distance` _player_location _enemy_location))
  (bind _returnvalue_2 (`KismetMathLibrary.MakeVector` (.x (/ (+ _player_location _enemy_location) 2)) (.y (/ (+ _player_location _enemy_location) 2)) (+ (.z (/ (+ _player_location _enemy_location) 2)) (`self.Camera Z Location`))))
  (bind (_returnvalue_roll _returnvalue_pitch _returnvalue_yaw) (`KismetMathLibrary.BreakRotator` (`KismetMathLibrary.FindLookAtRotation` (`self.K2_GetActorLocation`) _returnvalue_2)))
  (bind _returnvalue_3 (+ _returnvalue_2 (* (* (`KismetMathLibrary.GetForwardVector` (`self.Player Rotation`)) (`KismetMathLibrary.FClamp` _returnvalue (* _camera_length 2.0) (+ (/ _returnvalue 2.0) _camera_length))) (select `bool` (`self.Switch Camera Side`) :`false` -1 :`true` 1))))
  ;[1 1 1] Update Camera Location, Rotation & FOV
  (bind (_outhit _returnvalue_4) (`KismetSystemLibrary.LineTraceSingle` _returnvalue_2 _returnvalue_3 "TraceTypeQuery2" false (`|MakeArray` (`self.Player`) (`self.Enemy`) :!type "Actor Object Reference")))
  (`|ExecutionSequence`
    (:`then_0`
      (bind (_bblockinghit _binitialoverlap _time _distance _location _impactpoint) (`GameplayStatics.BreakHitResult` _outhit))
      (if (and _returnvalue_4 (< (`KismetMathLibrary.Vector_Distance` _impactpoint _returnvalue_3) (`self.Camera Length`)))
        (`self.Switch Camera`)))
    (:`then_1`
      (return (`KismetMathLibrary.VInterpTo` (`self.GetCameraLocation`) (select `bool` _returnvalue_4 :`false` _returnvalue_3 :`true` _impactpoint) (`GameplayStatics.GetWorldDeltaSeconds`) 10.0) (`KismetMathLibrary.RInterpTo` (`self.GetCameraRotation`) (`KismetMathLibrary.MakeRotator` 0.0 0.0 _returnvalue_yaw) (`GameplayStatics.GetWorldDeltaSeconds`) 10.0) 90.0 true))))

(fn `Camera Data`
  (returns (`Switch Camera` :type Boolean))
  (return (`self.Switch Camera Side`)))

(fn `Get Enemy Data`
  ;[1 1 1] Get Enemy Data
  (bind _enemy (`self.Enemy`)
    (:`then`
      (bind (_actor_rotation _actor_location) (message `/Game/Blueprints/Data/Interfaces/BP_CharacterData.Base Data` _enemy))
      (set `self.Enemy Location` _actor_location))
    (:`else`)))

(fn `Get Player Data`
  ;[1 1 1] Get Player Data
  (bind _player (`self.Player`)
    (:`then`
      (bind (_actor_rotation _actor_location) (message `/Game/Blueprints/Data/Interfaces/BP_CharacterData.Base Data` _player))
      (set `self.Player Rotation` _actor_rotation)
      (set `self.Player Location` (`KismetMathLibrary.MakeVector` (.x _actor_location) (.y _actor_location) (+ (.z _actor_location) 50.0))))
    (:`else`)))

(fn `Get Refs`
  ;[1 1 1] Get Refs
  (bind _asbp_player (cast `/Game/Blueprints/BP_Player` (`Controller.K2_GetPawn` (`self.GetOwningPlayerController`))))
  (bind _output_get (set `self.Player` _asbp_player))
  (bind (_game_instance _game_mode _game_state _player_controller _camera_manager _player_state _player _enemy) (message `/Game/Blueprints/Data/Interfaces/BP_GameData.Get Game Refs` _output_get))
  (set `self.Player Controller` _player_controller)
  (set `self.Enemy` _enemy))

(fn `UserConstructionScript`)