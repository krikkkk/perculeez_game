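; BP_Main_GameMode is the main game mode, running the fight start countdown and tracking game started, game ended and timer state.
; BeginPlay sets the texture streaming pool, caches the GameInstance, loads user settings and shows the WB_FightStart widget, whose animation-end callback starts the game.
; A Delay-loop macro counts the timer down and delays game end.
; GetGameModeData bundles this state with GameInstance fighting data; other getters are empty stubs.
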(event `self.ReceiveBeginPlay`
  ;[1 1 1] Begin Play
  (`|ExecutionSequence`
    (:`then_0`
      (`KismetSystemLibrary.ExecuteConsoleCommand` "r.streaming.poolsize 3000" null)
      (bind _asbp_main_game_instance (cast `/Game/Blueprints/Base/BP_Main_GameInstance` (`GameplayStatics.GetGameInstance`)))
      (set `self.Game Instance` _asbp_main_game_instance)
      (bind _returnvalue (`GameUserSettings.GetGameUserSettings`))
      (`GameUserSettings.LoadSettings` _returnvalue false))
    (:`then_1`
      (bind _returnvalue_2 (`|CreateWidget` "/Game/Blueprints/UI/GamePlay/Custom/WB_FightStart.WB_FightStart_C" null self))
      (bind _output_get (set `self.Start Fight Widget` _returnvalue_2))
      (`UserWidget.AddToViewport` _output_get 0)
      (`/Game/Blueprints/UI/GamePlay/Custom/WB_FightStart.Start UI Fight Animation` _output_get 3))))

(event `Fight UI Animation Ended`
  ;[1 1 1] Fight UI Animation Ended
  (set `self.Game Started` true)
  (bind _start_fight_widget (`self.Start Fight Widget`)
    (:`then`
      (`Widget.RemoveFromParent` _start_fight_widget))
    (:`else`)))

(event `Set Timer`
  (params (Timer :type Integer))
  ;[1 1 1] Set Timer
  (`self.Timer Macro` Timer))

(event `On Game Ends`
  ;[1 1 1] On Game Ends
  (`self.Timer Macro` 5
    (:`Completed`
      (set `self.Game Ended` true))))

(fn `Get Game Refs`
  (returns (`Game Instance` :type "/Game/Blueprints/Base/BP_Main_GameInstance Object Reference") (`Game Mode` :type "/Game/Blueprints/Base/GameMode/BP_Main_GameMode Object Reference") (`Game State` :type "/Game/Blueprints/Base/BP_Main_GameState Object Reference") (`Player Controller` :type "/Game/Blueprints/Base/BP_Main_PlayerController Object Reference") (`Camera Manager` :type "/Game/Blueprints/Base/BP_Main_CameraManager Object Reference") (`Player State` :type "/Game/Blueprints/Base/BP_Main_PlayerState Object Reference") (Player :type "/Game/Blueprints/BP_Player Object Reference") (Enemy :type "/Game/Blueprints/BP_Player Object Reference"))
  (return null null null null null null null null))

(fn `Get GameInstance data`
  (returns (`Fighting Data` :type "/Game/Blueprints/Data/Struc/S_Fighting_Data Structure"))
  (return))

(fn `Get GameMode Data`
  (returns (`Fighting Data` :type "/Game/Blueprints/Data/Struc/S_Fighting_Data Structure") (`Game Started` :type Boolean) (Timer :type Integer) (`Game Ended` :type Boolean))
  (bind _game_instance (`self.Game Instance`)
    (:`then`
      (bind _fighting_data (`/Game/Blueprints/Data/Interfaces/BP_GameData.Get GameInstance data` _game_instance))
      (return _fighting_data (`self.Game Started`) (`self.Timer`) (`self.Game Ended`)))
    (:`else`)))

(fn `Get GameState Data`
  (returns (`Game Time` :type "Timecode Structure"))
  (return))

(fn `UserConstructionScript`)